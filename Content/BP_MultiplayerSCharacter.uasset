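; Player character for a shooter, handling yaw-relative movement, halved-sensitivity look, counter-limited multi-jump, shooting and health.
; BeginPlay hides the mesh's weapon bone, spawns BP_Gun00 onto a hand-gun socket, adds the HUD and initializes health.
; Shoot input calls PullTrigger; landing resets the jump counter.
; Damage lowers and prints health, then calls Dead on BP_MultiplayerSPlayerController when health runs out.
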(event `InputAction|Jump`
  (params (Key :type "Key Structure"))
  (bind _jump_counter (`self.Jump Counter`))
  ;[0 0.107 0.4072] Double Jump
  (:`Pressed`
    (if (< _jump_counter (`self.Max Jumps`))
      (set `self.Jump Counter` (+ _jump_counter 1))
      (`self.Jump`)))
  (:`Released`
    (`self.StopJumping`)))

(event `self.ReceiveBeginPlay`
  (bind _mesh (`self.Mesh`))
  ;[1 1 1] Begin Play
  (`|ExecutionSequence`
    (:`then_0`
      ;[0.03536 0.651 0.2351] Show BP_Gun00
      (`SkinnedMeshComponent.HideBoneByName` _mesh "weapon_r" "PBO_None")
      ;;[0.6302 0.0462 0] TODO LOOK INTO THIS
      (bind _returnvalue (`|SpawnActorFromClass` "/Game/BP_Gun00.BP_Gun00_C" (`SceneComponent.GetSocketTransform` _mesh "Gun00Socket" "RTS_World") "Undefined" "OverrideRootScale" self null))
      (`self.K2_AttachToComponent` _returnvalue _mesh "Gun00Socket" "SnapToTarget" "SnapToTarget" "SnapToTarget" true))
    (:`then_1`
      ;[1 1 1] Widgets
      (bind _returnvalue_2 (`|CreateWidget` "/Game/WBP_HUD.WBP_HUD_C"))
      (`UserWidget.AddToViewport` _returnvalue_2 0))
    (:`then_2`
      (set `self.Health` 100.0))))

(event `InputAxis|MoveForward`
  (params (AxisValue :type "Float (single-precision)"))
  (bind (_returnvalue_roll _returnvalue_pitch _returnvalue_yaw) (`KismetMathLibrary.BreakRotator` (`self.GetControlRotation`)))
  ;[0 0.2629 1] Movement
  (`self.AddMovementInput` (`KismetMathLibrary.GetForwardVector` (`KismetMathLibrary.MakeRotator` 0.0 0.0 _returnvalue_yaw)) AxisValue))

(event `InputAxis|LookRight`
  (params (AxisValue :type "Float (single-precision)"))
  ;[0 0.2629 1] Movement
  (`self.AddControllerYawInput` (/ AxisValue 2.0)))

(event `self.OnLanded`
  (params (Hit :type "HitResult Structure (by ref)"))
  ;[0 0.107 0.4072] Double Jump
  (set `self.Jump Counter` 0))

(event `InputAxis|LookUp`
  (params (AxisValue :type "Float (single-precision)"))
  ;[0 0.2629 1] Movement
  (`self.AddControllerPitchInput` (/ AxisValue 2.0)))

(event `InputAxis|MoveRight`
  (params (AxisValue :type "Float (single-precision)"))
  (bind (_returnvalue_roll _returnvalue_pitch _returnvalue_yaw) (`KismetMathLibrary.BreakRotator` (`self.GetControlRotation`)))
  ;[0 0.2629 1] Movement
  (`self.AddMovementInput` (`KismetMathLibrary.GetRightVector` (`KismetMathLibrary.MakeRotator` 0.0 0.0 _returnvalue_yaw)) AxisValue))

(event `InputAction|Shoot`
  (params (Key :type "Key Structure"))
  (:`Pressed`
    (`self.Pull Trigger`)))

(event `self.ReceiveAnyDamage`
  (params (Damage :type "Float (single-precision)") (DamageType :type "DamageType Object Reference") (InstigatedBy :type "Controller Object Reference") (DamageCauser :type "Actor Object Reference"))
  (bind _returnvalue (- (`self.Health`) Damage))
  (bind _output_get (set `self.Health` _returnvalue))
  (`KismetSystemLibrary.PrintString` (`KismetStringLibrary.Conv_DoubleToString` _returnvalue))
  (if (<= _output_get 0.0)
    (bind _asbp_multiplayer_splayer_controller (cast `/Game/BP_MultiplayerSPlayerController` (`self.GetController`)))
    (`/Game/BP_MultiplayerSPlayerController.Dead` _asbp_multiplayer_splayer_controller)))

(fn `UserConstructionScript`)